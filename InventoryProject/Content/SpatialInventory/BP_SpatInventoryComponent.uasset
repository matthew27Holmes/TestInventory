(event `self.ReceiveBeginPlay`
  (bind _returnvalue (`|CreateWidget` "/Game/SpatialInventory/WBP_SpatInventory.WBP_SpatInventory_C" null self 50.0))
  (set `self.SpatInventory` _returnvalue)
  (`KismetArrayLibrary.Array_Resize` (`self.Items`) (* (`self.Colums`) (`self.Rows`))))

(event `Key|I`
  (params (Key :type "Key Structure"))
  (bind _returnvalue (`GameplayStatics.GetPlayerController` 0))
  (bind _spatinventory (`self.SpatInventory`))
  (bind _returnvalue_2 (`Widget.IsVisible` _spatinventory))
  (:`Pressed`
    (set `PlayerController.bShowMouseCursor` (not _returnvalue_2) _returnvalue)
    (if _returnvalue_2
      (`Widget.RemoveFromParent` _spatinventory)
      (`WidgetBlueprintLibrary.SetInputMode_GameOnly` _returnvalue)
      (else
        (`UserWidget.AddToViewport` _spatinventory 0)
        (`WidgetBlueprintLibrary.SetInputMode_GameAndUIEx` _returnvalue null)))))

(event `Key|E`
  (params (Key :type "Key Structure"))
  (bind _returnvalue (`Actor.K2_GetActorLocation` (`GameplayStatics.GetPlayerCharacter` 0)))
  (:`Pressed`
    (bind _outhit (`KismetSystemLibrary.SphereTraceSingle` :`Start` _returnvalue :`End` (- _returnvalue (0.0 0.0 65.0)) :`Radius` 120.0 :`TraceChannel` "TraceTypeQuery1" :`DrawDebugType` "ForDuration"))
    (bind _asbp_spat_item (cast `/Game/SpatialInventory/Items/BP_SpatItem` (`.HitActor` (`GameplayStatics.BreakHitResult` _outhit))))
    (bind _success (`self.TryAddItem` (`/Game/SpatialInventory/Items/BP_SpatItem.ItemObject` _asbp_spat_item)))
    (if _success
      (`Actor.K2_DestroyActor` _asbp_spat_item))))

(event `self.ReceiveTick`
  (params (DeltaSeconds :type "Float (single-precision)"))
  (if (`self.IsDirty`)
    (set `self.IsDirty` false)
    (`self.OnInventoryUpdate`)))

(fn `AddItemAt`
  (params (ItemObject :type "/Game/SpatialInventory/Items/U_SpatItemObject Object Reference") (TopLeftIndex :type Integer))
  (bind _tile (`self.ForEachIndex` ItemObject TopLeftIndex)
    (:`LoopBody`
      (`KismetArrayLibrary.Array_Set` (`self.Items`) (`self.TileToIndex` _tile) ItemObject))
    (:`Completed`
      (set `self.IsDirty` true))))

(fn `GetAllItems`
  (returns (AllItems :type "Map of /Game/SpatialInventory/Items/U_SpatItemObject Object Reference to /Game/SpatialInventory/S_Tile Structure"))
  (locals (AllItemsLoc :type "Map of /Game/SpatialInventory/Items/U_SpatItemObject Object Reference to /Game/SpatialInventory/S_Tile Structure") (CurrentItem :type "/Game/SpatialInventory/Items/U_SpatItemObject Object Reference"))
  (for (_array_element _array_index) (`self.Items`)
    (bind _output_get (set `local.CurrentItem` _array_element))
    (`/Engine/EditorBlueprintResources/StandardMacros.IsValid` _output_get
      (:`Is Valid`
        (if (not (`BlueprintMapLibrary.Map_Contains` (`local.AllItemsLoc`) _array_element))
          (`BlueprintMapLibrary.Map_Add` (`local.AllItemsLoc`) _array_element (`self.IndexToTile` _array_index))))))
  (return (`local.AllItemsLoc`)))

(fn `GetItemAtIndex`
  (params (Index :type Integer))
  (returns (IsValid :type Boolean) (ItemObject :type "/Game/SpatialInventory/Items/U_SpatItemObject Object Reference"))
  (if (`KismetArrayLibrary.Array_IsValidIndex` (`self.Items`) Index)
    (return true (`|GetArrayItem` (`self.Items`) Index))
    (else
      (return false null))))

(fn `IndexToTile`
  (params (Index :type Integer))
  (returns (Tile :type "/Game/SpatialInventory/S_Tile Structure"))
  (bind _colums (`self.Colums`))
  (return (make `/Game/SpatialInventory/S_Tile` (mod Index _colums) (/ Index _colums))))

(fn `IsRoomAvaliable`
  (params (ItemObject :type "/Game/SpatialInventory/Items/U_SpatItemObject Object Reference") (TopLeftIndex :type Integer))
  (returns (RoomAvaliable :type Boolean))
  (`|ExecutionSequence`
    (:`then_0`
      (bind _tile (`self.ForEachIndex` ItemObject TopLeftIndex)
        (:`LoopBody`
          (if (`self.IsTileValid` _tile)
            (bind (_isvalid _itemobject) (`self.GetItemAtIndex` (`self.TileToIndex` _tile)))
            (if (not (and _isvalid (not (`KismetSystemLibrary.IsValid` _itemobject))))
              (return false))
            (else
              (return false))))))
    (:`then_1`
      (return true))))

(fn `RemoveItem`
  (params (ItemObject :type "/Game/SpatialInventory/Items/U_SpatItemObject Object Reference"))
  (`/Engine/EditorBlueprintResources/StandardMacros.IsValid` ItemObject
    (:`Is Valid`
      (for (_array_element _array_index) (`self.Items`)
        (if (== _array_element ItemObject)
          (`KismetArrayLibrary.Array_Set` (`self.Items`) _array_index)
          (set `self.IsDirty` true))))))

(fn `TileToIndex`
  (params (Tile :type "/Game/SpatialInventory/S_Tile Structure"))
  (returns (Index :type Integer))
  (return (+ Tile_X_2_A355F45442D914EF242C0A8F55106848 (* Tile_Y_4_F7A3E83B4960D3578950619C37C9AAED (`self.Colums`)))))

(fn `TryAddItem`
  (params (ItemObject :type "/Game/SpatialInventory/Items/U_SpatItemObject Object Reference"))
  (returns (Success :type Boolean))
  (`/Engine/EditorBlueprintResources/StandardMacros.IsValid` ItemObject
    (:`Is Valid`
      (for (_ _array_index) (`self.Items`) :!label _label
        (bind _roomavaliable (`self.IsRoomAvaliable` (`local.ItemObject`) _array_index))
        (if _roomavaliable
          (`self.AddItemAt` (`local.ItemObject`) _array_index)
          (return true)))
      (`|ExecutionSequence`
        (:`then_0`
          (`/Engine/EditorBlueprintResources/StandardMacros.DoOnce` false
            (:`Completed`
              (`/Game/SpatialInventory/Items/U_SpatItemObject.Rotate` (`local.ItemObject`))
              (goto _label))))
        (:`then_1`
          (`/Game/SpatialInventory/Items/U_SpatItemObject.Rotate` (`local.ItemObject`))
          (return false))))
    (:`Is Not Valid`
      (return false))))